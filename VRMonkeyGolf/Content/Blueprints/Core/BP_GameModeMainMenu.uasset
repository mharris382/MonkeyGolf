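; Main menu game mode for the VR golf game that sets up the local player's profile and online session on BeginPlay.
; It casts the local pawn and its VRGolfPlayerState, then copies the active profile's name and ID from MGProfileSubsystem into the player state.
; It then logs in to VRGolfOnlineSubsystem using that profile name.
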(event EventBeginPlay
  (bind _returnvalue (Subsystems|GetMGProfileSubsystem))
  (bind _returnvalue_2 (Class|MGProfileSubsystem|GetActiveProfile _returnvalue))
  (Utilities|FlowControl|Sequence
    (:then_0
      ;[0.15 0.15 0.15 0.5] Ensure local player has profile assigned
      (bind _asbp_vrgolf_player_pawn (Utilities|Casting|CastToBP_VRGolfPlayerPawn (Game|Player|GetPlayerPawn 0)))
      (bind _output_get (Variables|Default|SetLocalPlayerPawn _asbp_vrgolf_player_pawn))
      (bind _asvrgolf_player_state (Utilities|Casting|CastToVRGolfPlayerState (Variables|/Script/Engine.Pawn|GetPlayerState _output_get)))
      (bind _output_get_2 (Variables|Default|SetLocalPlayerState _asvrgolf_player_state))
      (Class|VRGolfPlayerState|SetProfileIdentity _output_get_2 (Variables|/Script/VRGolfSave.MGProfileSaveGame|GetProfileName _returnvalue_2) (Variables|/Script/VRGolfSave.MGProfileSaveGame|GetProfileID _returnvalue_2)))
    (:then_1
      ;[0.15 0.15 0.15 0.5] Login to VRGolfOnline
      (Class|VRGolfOnlineSubsystem|Login (Subsystems|GetVRGolfOnlineSubsystem) (Variables|/Script/VRGolfSave.MGProfileSaveGame|GetProfileName (Class|MGProfileSubsystem|GetActiveProfile (Subsystems|GetMGProfileSubsystem)))))))

(fn ConstructionScript)